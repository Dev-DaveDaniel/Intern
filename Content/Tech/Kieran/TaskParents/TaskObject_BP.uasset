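; Parent task object that players interact with to complete an assigned task, taking its mesh and a random interaction method from the Tasks data table.
; Pressing checks the player's task list and any required held item, then runs press, hold, button-bash or press-wait-press logic, reporting success to the task manager.
; A Hold macro separates holds from taps using gates and a retriggerable delay.
; Overlap shows an interaction widget to players with the task.
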(event `self.ReceiveBeginPlay`
  (bind _returnvalue (`|GetDataTableRow` "/Game/Tech/Kieran/Tasks_DT.Tasks_DT" (`KismetStringLibrary.Conv_StringToName` (`|GetEnumeratorNameAsString` (`self.RelatedTask`))))
    (:`then`
      (bind _output_get (set `self.InteractionMethod` (`KismetArrayLibrary.Array_Random` (`.InteractMethod_67_A183326C4BE7D9453FF945BB0981AFCA` (break `/Game/Tech/Kieran/TaskDetails_Struct` _returnvalue)))))
      (`KismetSystemLibrary.PrintString` (`KismetStringLibrary.Concat_StrStr` (`KismetSystemLibrary.GetDisplayName` self) "interact method - " (`|GetEnumeratorNameAsString` _output_get))))))

(event `/Game/Tech/Interact_BPI.Pressed`
  (params (`Interacting Actor` :type "/Game/ThirdPerson/Blueprints/BP_ThirdPersonCharacter Object Reference"))
  (bind _taskstruct (`self.TaskStruct`))
  (bind _interacting_actor (`self.Interacting Actor`))
  (bind _interacting_actor_2 (`self.Interacting Actor`))
  (bind ((`WaitTimer_51_9BF6BA9F4107F2CA6314C29C652A0FD7` _waittimer) (`Waitpressestocomplete_53_BBDC23184DBC751AB564C19AC0487818` _waitpressestocomplete)) (break `/Game/Tech/Kieran/TaskDetails_Struct` (`self.TaskStruct`)))
  (bind (_name _id _staticmesh _interactmethod _priority_ _description _moneyearned _prioritymoneyearned _stresspertick _prioritystresspertick _requiresitem_ _itemtospawn) (break `/Game/Tech/Kieran/TaskDetails_Struct` _taskstruct))
  ;[1 1 1] Checks if player currently has the task associated with this object
  (set `self.Interacting Actor` `Interacting Actor`)
  (if (`self.CanBeUsed?`)
    (set `self.PlayerHasTask?` false)
    (set `self.TaskStruct` (struct))
    (for _array_element (`/Game/ThirdPerson/Blueprints/BP_ThirdPersonCharacter.Task List` `Interacting Actor`)
      (if (`|EnumEquality` (`self.RelatedTask`) (`.ID_18_952CBC6B46B80849CE80C7A1C83A99C9` (break `/Game/Tech/Kieran/TaskDetails_Struct` _array_element)))
        (set `self.PlayerHasTask?` true)
        (set `self.TaskStruct` _array_element)))
    ;[1 1 1] Checks if player has required task, and if the task requires an item that the player is holding it
    (if (`self.PlayerHasTask?`)
      (if _requiresitem_
        (if (== (`GameplayStatics.GetObjectClass` (`/Game/ThirdPerson/Blueprints/BP_ThirdPersonCharacter.HeldItem` _interacting_actor)) _itemtospawn)
          (bind _interactwidget (`self.InteractWidget` :!label _label)
            (:`then`
              (`/Game/Tech/Kieran/UI/Interact_Widget.UIInteract` _interactwidget _taskstruct))
            (:`else`
              _))
          (switch `/Game/Tech/Kieran/Enums/InteractType_Enum` (`self.InteractionMethod`)
            (:`NewEnumerator0`
              (`/Game/Tech/Kieran/TaskParents/TaskManager_BP.TaskComplete` (`self.TaskManagerRef`) _interacting_actor_2 (`self.RelatedTask`))
              (`/Game/Tech/Kieran/UI/Interact_Widget.E_PrintConfirmation` (`self.InteractWidget`) "PRESS SUCCESS")
              (`KismetSystemLibrary.Delay` 0.5)
              (`/Game/ThirdPerson/Blueprints/BP_ThirdPersonCharacter.DestroyTaskItem` _interacting_actor_2))
            (:`NewEnumerator1`
              ;[1 1 1] If player holds button for enough time, task is complete
              (set `self.CanBeUsed?` false)
              (`self.Hold?` (`.HoldTimer_52_43091D32496D9D3C27FFF398668112CC` (break `/Game/Tech/Kieran/TaskDetails_Struct` (`self.TaskStruct`))) :!label _label_2
                (:`Held`
                  (set `self.CanBeUsed?` true)
                  (`/Game/Tech/Kieran/TaskParents/TaskManager_BP.TaskComplete` (`self.TaskManagerRef`) (`self.Interacting Actor`) (`self.RelatedTask`))
                  (`/Game/Tech/Kieran/UI/Interact_Widget.E_PrintConfirmation` (`self.InteractWidget`) "HOLD SUCCESS")
                  (`/Game/ThirdPerson/Blueprints/BP_ThirdPersonCharacter.DestroyTaskItem` (`self.Interacting Actor`) :!label _label_3))
                (:`Tap`
                  (set `self.CanBeUsed?` true)
                  (`/Game/Tech/Kieran/UI/Interact_Widget.E_PrintConfirmation` (`self.InteractWidget`) "HOLD FAILURE"))))
            (:`NewEnumerator2`
              ;[1 1 1] Once pressed, increments bar until pressed enough times
              (bind _result (`/Engine/EditorBlueprintResources/StandardMacros.IncrementInt` (`self.TimesPressed`))
                (:`  `
                  (if (>= _result (`.BashpressesToComplete_55_F535FF914193C07257DCB588C5AF886B` (break `/Game/Tech/Kieran/TaskDetails_Struct` (`self.TaskStruct`))))
                    (set `self.TimesPressed` 0)
                    (`/Game/Tech/Kieran/TaskParents/TaskManager_BP.TaskComplete` (`self.TaskManagerRef`) (`self.Interacting Actor`) (`self.RelatedTask`))
                    (`/Game/Tech/Kieran/UI/Interact_Widget.E_PrintConfirmation` (`self.InteractWidget`) "BASH SUCCESS")
                    (goto _label_3)))))
            (:`NewEnumerator3`
              ;[1 1 1] Once pressed, prevents player from using for a short time until enough presses completed
              (set `self.CanBeUsed?` false)
              (bind _result_2 (`/Engine/EditorBlueprintResources/StandardMacros.IncrementInt` (`self.TimesPressed`))
                (:`  `
                  (if (>= _result_2 _waitpressestocomplete)
                    (set `self.CanBeUsed?` true)
                    (`/Game/Tech/Kieran/TaskParents/TaskManager_BP.TaskComplete` (`self.TaskManagerRef`) (`self.Interacting Actor`) (`self.RelatedTask`))
                    (`/Game/Tech/Kieran/UI/Interact_Widget.E_PrintConfirmation` (`self.InteractWidget`) "WAIT SUCCESS")
                    (goto _label_3)
                    (else
                      (`KismetSystemLibrary.Delay` _waittimer)
                      (set `self.CanBeUsed?` true))))))))
        (else
          (`/Game/ThirdPerson/Blueprints/BP_ThirdPersonCharacter.DropTaskItem` _interacting_actor)
          (goto _label))))))

(event `/Game/Tech/Interact_BPI.Released`
  (params (`Interacting Actor` :type "/Game/ThirdPerson/Blueprints/BP_ThirdPersonCharacter Object Reference"))
  ;[1 1 1] If player holds button for enough time, task is complete
  (goto _label_2 :!via `Released`))

(event `self.UICollision.OnComponentBeginOverlap`
  (params (OverlappedComponent :type "PrimitiveComponent Object Reference") (OtherActor :type "Actor Object Reference") (OtherComp :type "PrimitiveComponent Object Reference") (OtherBodyIndex :type Integer) (bFromSweep :type Boolean) (SweepResult :type "HitResult Structure (by ref)"))
  (`self.InteractWidget`
    (:`then`)
    (:`else`
      (bind _playerhastask_ (message `/Game/Tech/Kieran/Interfaces/Player_BPI.PlayerHasTask?` OtherActor (`self.RelatedTask`)))
      (if _playerhastask_
        (bind _controller (message `/Game/Tech/Kieran/Interfaces/Player_BPI.GetPlayerController` OtherActor))
        (bind _returnvalue (`|CreateWidget` "/Game/Tech/Kieran/UI/Interact_Widget.Interact_Widget_C" _controller (`self.InteractionMethod`)))
        (bind _output_get (set `self.InteractWidget` _returnvalue))
        (`UserWidget.AddToPlayerScreen` _output_get 0)))))

(event `self.UICollision.OnComponentEndOverlap`
  (params (OverlappedComponent :type "PrimitiveComponent Object Reference") (OtherActor :type "Actor Object Reference") (OtherComp :type "PrimitiveComponent Object Reference") (OtherBodyIndex :type Integer))
  (bind _interactwidget (`self.InteractWidget`)
    (:`then`
      (`Widget.RemoveFromParent` _interactwidget)
      (set `self.InteractWidget` null))
    (:`else`)))

(fn `UserConstructionScript`
  (`parent.UserConstructionScript`)
  (bind _returnvalue (`|GetDataTableRow` "/Game/Tech/Kieran/Tasks_DT.Tasks_DT" (`KismetStringLibrary.Conv_StringToName` (`|GetEnumeratorNameAsString` (`self.RelatedTask`))))
    (:`then`
      (`StaticMeshComponent.SetStaticMesh` (`self.Mesh`) (`.StaticMesh_58_8158B90543029F6953D171AB5746FC9B` (break `/Game/Tech/Kieran/TaskDetails_Struct` _returnvalue))))))