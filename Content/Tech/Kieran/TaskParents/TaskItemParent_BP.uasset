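; TaskItemParent_BP is a parent Blueprint for task items that a character can pick up and carry.
; On BeginPlay it passes its Icon to its widget component to show the task icon.
; When pressed, it makes the interacting actor drop any held task item, snaps itself to that actor's right-hand socket, registers as the held item and destroys the widget.
; GetIcon exposes the icon to other Blueprints.
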(event `self.ReceiveBeginPlay`
  ;[0.1818 0.5709 1] Platon
  (message `/Game/Tech/Kieran/Interfaces/Player_BPI.UpdateTaskIcon` (`WidgetComponent.GetUserWidgetObject` (`self.Widget`)) (`self.Icon`)))

(event `/Game/Tech/Interact_BPI.Pressed`
  (params (`Interacting Actor` :type "/Game/ThirdPerson/Blueprints/BP_ThirdPersonCharacter Object Reference"))
  (`/Game/ThirdPerson/Blueprints/BP_ThirdPersonCharacter.DropTaskItem` `Interacting Actor`)
  (`self.K2_AttachToActor` `Interacting Actor` "RHandSocket" "SnapToTarget" "SnapToTarget" "SnapToTarget")
  (`/Game/ThirdPerson/Blueprints/BP_ThirdPersonCharacter.SetHeldItem` `Interacting Actor` self)
  (`ActorComponent.K2_DestroyComponent` (`self.Widget`)))

(fn `GetIcon`
  (returns (Texture :type "Texture Object Reference"))
  (return (`self.Icon`)))

(fn `UserConstructionScript`
  (`parent.UserConstructionScript`))