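; Parent Blueprint for destructible task objects that reward the player who breaks them with cash and stress reduction.
; SetDestroyer stores the player, removes the static mesh, makes the geometry collection block all channels and fires a particle effect.
; The first Chaos break event with a valid destroyer plays a hit sound, messages that player with both values, then destroys the actor after a short delay.
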(event `/Game/Tech/Kieran/Interfaces/Destructible_BPI.SetDestroyer`
  (params (Destroyer :type "Actor Object Reference"))
  (bind _staticmesh (`self.StaticMesh`))
  (set `self.DestroyingPlayer` Destroyer)
  (`/Engine/EditorBlueprintResources/StandardMacros.IsValid` _staticmesh
    (:`Is Valid`
      (`ActorComponent.K2_DestroyComponent` _staticmesh))
    (:`Is Not Valid`
      _))
  (`PrimitiveComponent.SetCollisionResponseToAllChannels` (`self.GeometryCollection`) "ECR_Block")
  (`ActorComponent.Activate` (`self.ParticleEffect`) false))

(event `self.GeometryCollection.OnChaosBreakEvent`
  (params (BreakEvent :type "ChaosBreakEvent Structure (by ref)"))
  (bind _destroyingplayer (`self.DestroyingPlayer`))
  (`/Engine/EditorBlueprintResources/StandardMacros.IsValid` (`self.DestroyingPlayer`)
    (:`Is Valid`
      (`/Engine/EditorBlueprintResources/StandardMacros.DoOnce` false
        (:`Completed`
          (`GameplayStatics.PlaySoundAtLocation` "/Game/Design/Sound/Hit2_SFX.Hit2_SFX" (`self.K2_GetActorLocation`) (struct) 1.0 1.0 0.0 null null null null)
          (`KismetSystemLibrary.PrintString` (`KismetSystemLibrary.GetDisplayName` _destroyingplayer))
          (message `/Game/Tech/Kieran/Interfaces/Destructible_BPI.ItemDestroyed` _destroyingplayer (`self.CashValue`) (`self.StressReduction`))
          (`KismetSystemLibrary.Delay` 5.0)
          (`self.K2_DestroyActor`))))))

(fn `UserConstructionScript`)