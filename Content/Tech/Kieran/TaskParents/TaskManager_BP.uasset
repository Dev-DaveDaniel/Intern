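; Task manager that hands out random tasks to players on a looping timer and stops it at Post-Game.
; Each tick, players with under five tasks get a Tasks_DT row matching a level task object, rerolled until valid and not already held, with random priority.
; Assignment highlights a matching object and spawns any required item at a free spawn area.
; Completion pays normal or priority cash, removes the task and clears highlights nobody still needs.
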(event `/Game/Tech/Kieran/Interfaces/GameState_BPI.ChangeState`
  (params (NewState :type "/Game/Tech/Kieran/Enums/GameState_Enum Enum" :default "NewEnumerator0"))
  (switch `/Game/Tech/Kieran/Enums/GameState_Enum` NewState
    (:`NewEnumerator3`
      (`KismetSystemLibrary.K2_ClearAndInvalidateTimerHandle` (`self.TaskTimerHandle`)))))

(event `/Game/Tech/Kieran/Interfaces/Initialize_BPI.Initialize`
  ;[1 1 1] Add all players to array on begin play
  (bind _outactors (`GameplayStatics.GetAllActorsOfClass` "/Game/Tech/Kieran/TaskParents/TaskObject_BP.TaskObject_BP_C"))
  (for _array_element _outactors
    (`KismetArrayLibrary.Array_AddUnique` (`self.UsableTasks`) (`/Game/Tech/Kieran/TaskParents/TaskObject_BP.RelatedTask` _array_element)))
  (bind _outactors_2 (`GameplayStatics.GetAllActorsOfClass` "/Game/ThirdPerson/Blueprints/BP_ThirdPersonCharacter.BP_ThirdPersonCharacter_C"))
  (set `self.PlayerCharacters` _outactors_2)
  (bind _outactors_3 (`GameplayStatics.GetAllActorsOfClass` "/Game/Tech/Kieran/TaskParents/TaskItemSpawner_BP.TaskItemSpawner_BP_C"))
  (set `self.ItemSpawnAreas` _outactors_3)
  (bind _outactors_4 (`GameplayStatics.GetAllActorsOfClass` "/Game/Tech/Kieran/TaskParents/TaskObject_BP.TaskObject_BP_C"))
  (bind _output_get (set `self.TaskObjectList` _outactors_4))
  (for _array_element_2 _output_get
    (set `/Game/Tech/Kieran/TaskParents/TaskObject_BP.TaskManagerRef` self _array_element_2))
  (add `self.TaskComplete` (delegate `CompletedTask`))
  ;[1 1 1] Sets timer based on Task Timer and assigns all players a task each tick of this timer
  (bind _returnvalue (`KismetSystemLibrary.K2_SetTimerDelegate` (delegate `AssignTask`) (`self.TaskTimer`) true))
  (set `self.TaskTimerHandle` _returnvalue))

(event `AssignTask`
  ;[1 1 1] Sets timer based on Task Timer and assigns all players a task each tick of this timer
  (`KismetArrayLibrary.Array_Clear` (`self.NeedsTask`))
  (for _array_element (`self.PlayerCharacters`)
    (if (not (>= (`KismetArrayLibrary.Array_Length` (`/Game/ThirdPerson/Blueprints/BP_ThirdPersonCharacter.Task List` _array_element)) 5))
      (`KismetArrayLibrary.Array_Add` (`self.NeedsTask`) _array_element)))
  (if (> (`KismetArrayLibrary.Array_Length` (`self.NeedsTask`)) 0)
    ;[1 1 1] Generates random number and finds corresponding task in data table. Checks if player has task already. If not, gives player task in their own array. If they do, loops until player assigned new task
    (for _array_element_2 (`self.NeedsTask`) :!label _label
      (set `self.HasTask?` false)
      (bind _returnvalue (`|GetDataTableRow` "/Game/Tech/Kieran/Tasks_DT.Tasks_DT" (`KismetStringLibrary.Conv_StringToName` (`KismetStringLibrary.Conv_IntToString` (`KismetMathLibrary.RandomIntegerInRange` 1 (`self.NumberOfTasks`)))))
        (:`then`
          (bind (_name _id _staticmesh _interactmethod _priority_ _description _moneyearned _prioritymoneyearned _stresspertick _prioritystresspertick _requiresitem_ _itemtospawn _itemicon _bashpressestocomplete _holdtimer _waittimer _waitpressestocomplete) (break `/Game/Tech/Kieran/TaskDetails_Struct` _returnvalue))
          (bind _returnvalue_2 (`KismetArrayLibrary.Array_Contains` (`self.UsableTasks`) _id))
          (if _returnvalue_2
            (`KismetSystemLibrary.PrintString` (`KismetStringLibrary.Conv_BoolToString` _returnvalue_2))
            (bind _task_list (`/Game/ThirdPerson/Blueprints/BP_ThirdPersonCharacter.Task List` _array_element_2))
            (if (== (`KismetArrayLibrary.Array_Length` _task_list) 0)
              (bind _taskdetails_struct (make `/Game/Tech/Kieran/TaskDetails_Struct` _name _id _staticmesh _interactmethod (<= (`KismetMathLibrary.RandomIntegerInRange` 1 100) (`self.Priority Chance %`)) _description _moneyearned 0.0 _stresspertick 0.0 _requiresitem_ _itemtospawn null _bashpressestocomplete _holdtimer _waittimer _waitpressestocomplete))
              (`/Game/ThirdPerson/Blueprints/BP_ThirdPersonCharacter.AddTask` _array_element_2 _taskdetails_struct :!label _label_2)
              (`KismetArrayLibrary.Array_RemoveItem` (`self.NeedsTask`) _array_element_2)
              (bind ((`ID_18_952CBC6B46B80849CE80C7A1C83A99C9` _id_2) (`RequiresItem?_60_192C792A47EF89AFA67A4890F4E09B44` _requiresitem__2)) (break `/Game/Tech/Kieran/TaskDetails_Struct` _returnvalue))
              (if _requiresitem__2
                (`self.SpawnRelatedActors` _taskdetails_struct))
              (`self.SetHighlight` _taskdetails_struct)
              (else
                (for _array_element_3 _task_list
                  (if (`|EnumEquality` _id_2 (`.ID_18_952CBC6B46B80849CE80C7A1C83A99C9` (break `/Game/Tech/Kieran/TaskDetails_Struct` _array_element_3)))
                    (set `self.HasTask?` true)))
                (if (not (`self.HasTask?`))
                  (goto _label_2))))))))
    (if (> (`KismetArrayLibrary.Array_Length` (`self.NeedsTask`)) 0)
      (goto _label))))

(event `CompletedTask` :!signature `self.TaskComplete`
  (params (`Completing Actor` :type "/Game/ThirdPerson/Blueprints/BP_ThirdPersonCharacter Object Reference") (`Completed Task` :type "/Game/Tech/Kieran/Enums/TaskID_Enum Enum" :default "NewEnumerator0"))
  (`self.TaskCompleted` `Completing Actor` `Completed Task`))

(event `self.ReceiveBeginPlay`
  (`KismetSystemLibrary.Delay` 0.2))

(fn `ChooseMap`
  (returns (Name :type Name))
  (return "None"))

(fn `SetHighlight`
  (params (TaskDetails :type "/Game/Tech/Kieran/TaskDetails_Struct Structure"))
  (bind _outactors (`GameplayStatics.GetAllActorsOfClass` "/Game/Tech/Kieran/TaskParents/TaskObject_BP.TaskObject_BP_C"))
  (for _array_element _outactors
    (if (`|EnumEquality` (`/Game/Tech/Kieran/TaskParents/TaskObject_BP.RelatedTask` _array_element) (`.ID_18_952CBC6B46B80849CE80C7A1C83A99C9` (break `/Game/Tech/Kieran/TaskDetails_Struct` TaskDetails)))
      (`/Game/Tech/Kieran/TaskParents/TaskObject_BP.AddHighlight` _array_element)
      (break))))

(fn `SpawnRelatedActors`
  (params (Task :type "/Game/Tech/Kieran/TaskDetails_Struct Structure"))
  (bind ((`InteractMethod_67_A183326C4BE7D9453FF945BB0981AFCA` _interactmethod) (`PriorityMoneyearned_72_3B61D0174F89A1587B28068EA81A0296` _prioritymoneyearned) (`PriorityStresspertick_73_3FECCDF54A7CBBDC9893E48C59C6245B` _prioritystresspertick) (`ItemToSpawn_61_641E80424933AEFC1D6A618C06E195F6` _itemtospawn)) (break `/Game/Tech/Kieran/TaskDetails_Struct` Task))
  ;[1 1 1] If task has item associated with it, spawns that item at an available item spawn zone
  (for _array_element (`self.ItemSpawnAreas`)
    (if (not (`/Game/Tech/Kieran/TaskParents/TaskItemSpawner_BP.InUse?` _array_element))
      (`|SpawnActorFromClass` _itemtospawn (`self.GetTransform` _array_element) "AlwaysSpawn" "OverrideRootScale" null null null)
      (set `/Game/Tech/Kieran/TaskParents/TaskItemSpawner_BP.InUse?` true _array_element)
      (set `/Game/Tech/Kieran/TaskParents/TaskItemSpawner_BP.ItemInArea` _itemtospawn _array_element)
      (break))))

(fn `TaskCompleted`
  (params (Player :type "/Game/ThirdPerson/Blueprints/BP_ThirdPersonCharacter Object Reference") (TaskID :type "/Game/Tech/Kieran/Enums/TaskID_Enum Enum" :default "NewEnumerator0"))
  (locals (`L CompletedTask` :type "/Game/Tech/Kieran/TaskDetails_Struct Structure") (CashEarned :type "Float (double-precision)") (`KeepHighlight?` :type Boolean))
  (bind _l_completedtask (`local.L CompletedTask`))
  (bind _task_list (`/Game/ThirdPerson/Blueprints/BP_ThirdPersonCharacter.Task List` Player))
  (bind (_name _id _staticmesh _interactmethod _priority_ _description _moneyearned _prioritymoneyearned) (break `/Game/Tech/Kieran/TaskDetails_Struct` _l_completedtask))
  ;[1 1 1] Finds task in player task list and removes it from their list
  (for _array_element _task_list
    (if (`|EnumEquality` (`.ID_18_952CBC6B46B80849CE80C7A1C83A99C9` (break `/Game/Tech/Kieran/TaskDetails_Struct` _array_element)) TaskID)
      (set `local.L CompletedTask` _array_element)))
  (`/Game/ThirdPerson/Blueprints/BP_ThirdPersonCharacter.GainCash` Player (`KismetMathLibrary.SelectFloat` _prioritymoneyearned _moneyearned _priority_))
  (`/Game/ThirdPerson/Blueprints/BP_ThirdPersonCharacter.RemoveTask` Player _l_completedtask)
  (`KismetArrayLibrary.Array_RemoveItem` _task_list _l_completedtask)
  (bind _outactors (`GameplayStatics.GetAllActorsOfClass` "/Game/ThirdPerson/Blueprints/BP_ThirdPersonCharacter.BP_ThirdPersonCharacter_C"))
  (for _array_element_2 _outactors :!label _label
    (for _array_element_3 (`/Game/ThirdPerson/Blueprints/BP_ThirdPersonCharacter.Task List` _array_element_2)
      (if (`|EnumEquality` (`.ID_18_952CBC6B46B80849CE80C7A1C83A99C9` (break `/Game/Tech/Kieran/TaskDetails_Struct` _array_element_3)) _id)
        (set `local.KeepHighlight?` true)
        (goto _label :!via `Break`))))
  (if (not (`local.KeepHighlight?`))
    (bind _outactors_2 (`GameplayStatics.GetAllActorsOfClass` "/Game/Tech/Kieran/TaskParents/TaskObject_BP.TaskObject_BP_C"))
    (for _array_element_4 _outactors_2
      (if (`|EnumEquality` (`/Game/Tech/Kieran/TaskParents/TaskObject_BP.RelatedTask` _array_element_4) (`.ID_18_952CBC6B46B80849CE80C7A1C83A99C9` (break `/Game/Tech/Kieran/TaskDetails_Struct` (`local.L CompletedTask`))))
        (`/Game/Tech/Kieran/TaskParents/TaskObject_BP.RemoveHighlight` _array_element_4)))
    (return)))

(fn `UserConstructionScript`)