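; Toaster toy actor that launches two physics meshes, presumably toast slices, when its Pressed event fires.
; Pressing makes both meshes visible, enables their physics simulation, activates two physics thrusters and repositions a third mesh.
; A brief delay then deactivates the thrusters, so the launch is a short impulse-like burst.
; Nothing in the graph resets the toaster afterwards.
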(event `/Game/Tech/Interact_BPI.Pressed`
  (params (`Interacting Actor` :type "/Game/ThirdPerson/Blueprints/BP_ThirdPersonCharacter Object Reference"))
  (`SceneComponent.SetVisibility` (`self.StaticMesh1`) true false)
  (`SceneComponent.SetVisibility` (`self.StaticMesh2`) true false)
  (`PrimitiveComponent.SetSimulatePhysics` (`self.StaticMesh1`) true)
  (`PrimitiveComponent.SetSimulatePhysics` (`self.StaticMesh2`) true)
  (`ActorComponent.SetActive` (`self.PhysicsThruster`) true false)
  (`ActorComponent.SetActive` (`self.PhysicsThruster1`) true false)
  (`SceneComponent.K2_SetRelativeLocation` (`self.StaticMesh`) (0.0 0.0 8.0) false false)
  (`KismetSystemLibrary.Delay` 0.05)
  (`ActorComponent.Deactivate` (`self.PhysicsThruster`))
  (`ActorComponent.Deactivate` (`self.PhysicsThruster1`)))

(fn `UserConstructionScript`
  (`parent.UserConstructionScript`))