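; Fire extinguisher rocket toy Blueprint that turns into a propelled object when SetDestroyer is triggered.
; SetDestroyer activates a Niagara effect and a PhysicsThruster together, then shuts both off after a four-second delay.
; The construction script only runs the parent's, so other behavior comes from the parent class.
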(event `/Game/Tech/Kieran/Interfaces/Destructible_BPI.SetDestroyer`
  (params (Destroyer :type "Actor Object Reference"))
  (`ActorComponent.Activate` (`self.Niagara`) false)
  (`ActorComponent.Activate` (`self.PhysicsThruster`) false)
  (`KismetSystemLibrary.Delay` 4.0)
  (`ActorComponent.Deactivate` (`self.Niagara`))
  (`ActorComponent.Deactivate` (`self.PhysicsThruster`)))

(fn `UserConstructionScript`
  (`parent.UserConstructionScript`))