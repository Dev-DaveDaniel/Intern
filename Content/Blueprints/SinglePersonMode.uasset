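; Single-player game mode that spawns and possesses a third-person character at random BP_SpawnActor points and switches the view to fixed cameras, ending BeginPlay on a CCTV camera.
; TaskCreator picks one of five random chore tasks, fires a dispatcher and re-arms its own looping timer.
; StartTask is empty and the "Tasks Begin" branch is unconnected, so nothing here starts the task cycle.
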(event `Setup Camera`
  (bind _returnvalue (`GameplayStatics.GetActorOfClass` "/Game/Design/Wyn/Cameras/CCTVCamera.CCTVCamera_C"))
  (`PlayerController.SetViewTargetWithBlend` (`GameplayStatics.GetPlayerController` 0) _returnvalue 0.0 "VTBlend_Linear" 0.0 false))

(event `self.HandleStartingNewPlayer`
  (params (NewPlayer :type "PlayerController Object Reference"))
  (bind _returnvalue (`self.K2_FindPlayerStart` NewPlayer))
  (bind _returnvalue_2 (`|SpawnActorFromClass` "/Game/ThirdPerson/Blueprints/BP_ThirdPersonCharacter.BP_ThirdPersonCharacter_C" (`KismetMathLibrary.MakeTransform` (`self.K2_GetActorLocation` _returnvalue) (`self.K2_GetActorRotation` _returnvalue)) "Undefined" "OverrideRootScale" null null))
  (`Controller.Possess` NewPlayer _returnvalue_2)
  (`PlayerController.SetViewTargetWithBlend` (`GameplayStatics.GetPlayerController` 0) (`self.StartingCamera`) 0.0 "VTBlend_Linear" 0.0 false))

(event `self.ReceiveBeginPlay`
  (for _index (range 1)
    (bind _output_get (set `self.PlayerIndex` _index))
    (`GameplayStatics.CreatePlayer` _output_get)
    (`self.Setup Camera`)
    (`self.Start Task`)))

(event `Start Task`)

(event `TaskCreator`
  (set `self.TaskTime` 120.0)
  (bind _output_get (set `self.TasksEnum` (cast `/Game/Blueprints/Tasks` (`KismetMathLibrary.Conv_IntToByte` (`KismetMathLibrary.RandomIntegerInRange` 0 4)))))
  (switch `/Game/Blueprints/Tasks` _output_get
    (:`NewEnumerator0`
      (`KismetSystemLibrary.PrintString` "Task1"))
    (:`NewEnumerator1`
      (`KismetSystemLibrary.PrintString` "Task2"))
    (:`NewEnumerator2`
      (`KismetSystemLibrary.PrintString` "Task3"))
    (:`NewEnumerator3`
      (`KismetSystemLibrary.PrintString` "Task4"))
    (:`NewEnumerator4`
      (`KismetSystemLibrary.PrintString` "Task5")))
  (`self.TaskDispatcher`)
  (`KismetSystemLibrary.K2_ClearAndInvalidateTimerHandle` (stale _returnvalue))
  (set `self.TaskPresented?` true)
  (bind _returnvalue (`KismetSystemLibrary.K2_SetTimerDelegate` (delegate `TaskCreator`) (`self.TaskTime`) true)))

(fn `FindPlayerStart`
  (params (Player :type "Controller Object Reference") (IncomingName :type String))
  (returns (ReturnValue :type "Actor Object Reference"))
  (bind _outitem (`KismetArrayLibrary.Array_Random` (`self.SpawnPoints`)))
  (`/Engine/EditorBlueprintResources/StandardMacros.IsValid` _outitem
    (:`Is Valid`
      (return _outitem))
    (:`Is Not Valid`
      (return self))))

(fn `UserConstructionScript`
  (`KismetArrayLibrary.Array_Clear` (`self.SpawnPoints`))
  (bind _outactors (`GameplayStatics.GetAllActorsOfClass` "/Game/Blueprints/BP_SpawnActor.BP_SpawnActor_C"))
  (set `self.SpawnPoints` _outactors))