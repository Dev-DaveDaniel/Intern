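; Coffee delivery task actor in which the player collects beans at one trigger and brings them to another to win.
; StartCoffeeTask arms the task, then a sphere overlap by the third-person character sets a holding-beans flag.
; A box overlap while holding beans only prints a win message, without resetting either flag.
; The construction script caches the beans' world transform, which is not used elsewhere here.
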(event `Start Coffee Task`
  (set `self.IsCoffeeTaskActive?` true))

(event `self.Sphere.OnComponentBeginOverlap`
  (params (OverlappedComponent :type "PrimitiveComponent Object Reference") (OtherActor :type "Actor Object Reference") (OtherComp :type "PrimitiveComponent Object Reference") (OtherBodyIndex :type Integer) (bFromSweep :type Boolean) (SweepResult :type "HitResult Structure (by ref)"))
  (if (`self.IsCoffeeTaskActive?`)
    (cast `/Game/ThirdPerson/Blueprints/BP_ThirdPersonCharacter` OtherActor)
    (set `self.IsHoldingBeans?` true)
    (else
      (`KismetSystemLibrary.PrintString` "Task Not Active" true true (struct :`R` 1.0 :`G` 0.077069 :`A` 1.0)))))

(event `self.Box.OnComponentBeginOverlap`
  (params (OverlappedComponent :type "PrimitiveComponent Object Reference") (OtherActor :type "Actor Object Reference") (OtherComp :type "PrimitiveComponent Object Reference") (OtherBodyIndex :type Integer) (bFromSweep :type Boolean) (SweepResult :type "HitResult Structure (by ref)"))
  (if (`self.IsCoffeeTaskActive?`)
    (cast `/Game/ThirdPerson/Blueprints/BP_ThirdPersonCharacter` OtherActor)
    (if (`self.IsHoldingBeans?`)
      (`KismetSystemLibrary.PrintString` "Task Won"))))

(fn `UserConstructionScript`
  (set `self.CoffeeTransform` (`SceneComponent.K2_GetComponentToWorld` (`self.CoffeeBeans`))))